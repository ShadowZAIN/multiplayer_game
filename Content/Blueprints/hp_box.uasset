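; Health pickup box that restores a fixed amount of health to a FirstPersonCharacter overlapping it.
; The Box overlap event casts to the character, passes a DoOnce gate, then calls AddHealth on its BPCHealth component and hides the Box.
; After a delay, a Reset event shows the Box again and reopens the gate, making the pickup reusable.
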(event `self.box.OnComponentBeginOverlap`
  (params (OverlappedComponent :type "PrimitiveComponent Object Reference") (OtherActor :type "Actor Object Reference") (OtherComp :type "PrimitiveComponent Object Reference") (OtherBodyIndex :type Integer) (bFromSweep :type Boolean) (SweepResult :type "HitResult Structure (by ref)"))
  (bind _asfirst_person_character (cast `/Game/Blueprints/FirstPersonCharacter` OtherActor))
  (`/Engine/EditorBlueprintResources/StandardMacros.DoOnce` false :!label _label
    (:`Completed`
      (`/Game/Blueprints/Components/BPC_Health.AddHealth` (`/Game/Blueprints/FirstPersonCharacter.BPC_Health` _asfirst_person_character) 50.0)
      (`SceneComponent.SetVisibility` (`self.box`) false false)
      (`KismetSystemLibrary.Delay` 10.0)
      (`self.Reset`))))

(event `Reset`
  (`SceneComponent.SetVisibility` (`self.box`) true false)
  (goto _label :!via `Reset`))

(fn `UserConstructionScript`)