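; FPS player controller that handles the pause menu and the player's death and respawn cycle.
; The Menu input toggles a lazily created PauseMenu widget, switching pawn input, input mode and mouse cursor.
; Death destroys the pawn and possesses a spectator pawn spawned at the LevelCamera found on BeginPlay.
; A five-second timer then calls Respawn, which replaces the spectator with a new FirstPersonCharacter at a random PlayerStart.
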(event `self.ReceiveBeginPlay`
  (bind _outactors (`GameplayStatics.GetAllActorsOfClass` "/Game/Blueprints/LevelCamera.LevelCamera_C"))
  (set `self.Level Camera` (`|GetArrayItem` _outactors)))

(event `InputAction|Menu` :paused true
  (params (Key :type "Key Structure"))
  (:`Pressed`
    (`/Engine/EditorBlueprintResources/StandardMacros.IsValid` (`self.Menu`)
      (:`Is Valid`
        (if (`Widget.IsInViewport` (`self.Menu`))
          (`Widget.RemoveFromParent` (stale _output_get))
          (set `self.bShowMouseCursor` false)
          (`self.EnableInput` (`self.K2_GetPawn`) self)
          (`WidgetBlueprintLibrary.SetInputMode_GameOnly` self)
          (else
            (`UserWidget.AddToViewport` (stale _output_get) 0 :!label _label)
            (`self.DisableInput` (`self.K2_GetPawn`) self)
            (`WidgetBlueprintLibrary.SetInputMode_GameAndUIEx` self (`self.Menu`))
            (set `self.bShowMouseCursor` true))))
      (:`Is Not Valid`
        (bind _returnvalue (`|CreateWidget` "/Game/UI/PauseMenu.PauseMenu_C" self))
        (bind _output_get (set `self.Menu` _returnvalue))
        (goto _label)))))

(fn `Death`
  (`self.K2_DestroyActor` (`self.K2_GetPawn`))
  (bind _returnvalue (`|SpawnActorFromClass` "/Game/Blueprints/FPS_SpectatorPawn.FPS_SpectatorPawn_C" (`self.GetTransform` (`self.Level Camera`)) "Undefined" "OverrideRootScale" null null))
  (`self.Possess` _returnvalue)
  (`KismetSystemLibrary.K2_SetTimer` self "Respawn" 5.0))

(fn `Respawn`
  (`self.K2_DestroyActor` (`self.K2_GetPawn`))
  (bind _outactors (`GameplayStatics.GetAllActorsOfClass` "/Script/Engine.PlayerStart"))
  (bind _returnvalue (`|SpawnActorFromClass` "/Game/Blueprints/FirstPersonCharacter.FirstPersonCharacter_C" (`self.GetTransform` (`|GetArrayItem` _outactors (`KismetMathLibrary.RandomIntegerInRange` 0 (- (`KismetArrayLibrary.Array_Length` _outactors) 1)))) "Undefined" "OverrideRootScale" null null))
  (`self.Possess` _returnvalue))

(fn `UserConstructionScript`)