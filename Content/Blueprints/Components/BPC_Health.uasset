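; BPC_Health is a health component that tracks Health against MaxHealth and exposes getters for the current value and the dead state.
; AddHealth, Damage and Recovery change Health within its limits (heal capped at MaxHealth, damage floored at zero, Recovery refills fully) and each calls Update.
; Damage also calls OnDead whenever Health is zero afterwards, including on repeated hits.
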(fn `AddHealth`
  (params (Heal :type "Float (double-precision)"))
  (set `self.Health` (`KismetMathLibrary.FMin` (+ Heal (`self.Health`)) (`self.MaxHealth`)))
  (`self.Update`))

(fn `Damage`
  (params (Damage :type "Float (double-precision)"))
  (bind _output_get (set `self.Health` (`KismetMathLibrary.FMax` (- (`self.Health`) (`local.Damage`)))))
  (`self.Update`)
  (if (== _output_get 0.0)
    (`self.OnDead`)))

(fn `GetHealth`
  (returns (Health :type "Float (double-precision)"))
  (return (`self.Health`)))

(fn `IsDead?`
  (returns (Dead :type Boolean))
  (return (== (`self.Health`) 0.0)))

(fn `Recovery`
  (set `self.Health` (`self.MaxHealth`))
  (`self.Update`))