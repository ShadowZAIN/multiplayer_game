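; FPSController is a controller Blueprint that toggles the pause menu on the Menu input action.
; It creates the PauseMenu widget on first use, caches it, then adds it to or removes it from the viewport on each press.
; Showing the menu disables pawn input, switches to Game and UI input mode and shows the cursor; hiding it reverses these, without pausing the game.
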(event `InputAction|Menu` :paused true
  (params (Key :type "Key Structure"))
  (bind _returnvalue (`GameplayStatics.GetPlayerController` 0))
  (bind _returnvalue_2 (`GameplayStatics.GetPlayerController` 0))
  (:`Pressed`
    (`/Engine/EditorBlueprintResources/StandardMacros.IsValid` (`self.Menu`)
      (:`Is Valid`
        (if (`Widget.IsInViewport` (`self.Menu`))
          (`Widget.RemoveFromParent` (stale _output_get))
          (set `PlayerController.bShowMouseCursor` false _returnvalue_2)
          (`self.EnableInput` (`GameplayStatics.GetPlayerPawn` 0) _returnvalue_2)
          (`WidgetBlueprintLibrary.SetInputMode_GameOnly` _returnvalue_2)
          (else
            (`UserWidget.AddToViewport` (stale _output_get) 0 :!label _label)
            (`self.DisableInput` (`GameplayStatics.GetPlayerPawn` 0) _returnvalue)
            (`WidgetBlueprintLibrary.SetInputMode_GameAndUIEx` _returnvalue (`self.Menu`))
            (set `PlayerController.bShowMouseCursor` true _returnvalue))))
      (:`Is Not Valid`
        (bind _returnvalue_3 (`|CreateWidget` "/Game/UI/PauseMenu.PauseMenu_C" (`GameplayStatics.GetPlayerController` 0)))
        (bind _output_get (set `self.Menu` _returnvalue_3))
        (goto _label)))))

(fn `UserConstructionScript`)